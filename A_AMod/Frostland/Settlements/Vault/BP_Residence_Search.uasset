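; Scripted logic for the Vault settlement in the Frostland that reacts when the final residence search outpost runs out.
; On start it binds to the extraction subsystem's depletion update event.
; When the searching outpost is depleted, it spawns the residence-accessed dilemma at the outpost owner's transform, then destroys the outpost.
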(event `self.ReceiveStarted`
  (add `PXExtractionSubsystem.ExtractionDepletionUpdated` (subsystem `PXExtractionSubsystem`) (`|CreateDelegate` :!event `Residence Searched`)))

(event `Residence Searched`
  (params (extraction :type "PXExtractionComponent Object Reference"))
  (bind _returnvalue (`PXOutpostUtils.GetOutpostOfType` "/Game/Scenarios/Shared/Configs/A_AMod/Frostland/Settlements/Vault/Fixed/DA_Residence_Searching_Final.DA_Residence_Searching_Final"))
  (if (`PXOutpostUtils.IsOutpostDepleted` (`PXOutpostUtils.GetOutpostOfType` "/Game/Scenarios/Shared/Configs/A_AMod/Frostland/Settlements/Vault/Fixed/DA_Residence_Searching_Final.DA_Residence_Searching_Final"))
    (`PXDilemmaUtils.SpawnDilemma` (`Actor.GetTransform` (`ActorComponent.GetOwner` _returnvalue)) "/Game/Scenarios/Shared/Configs/A_AMod/Frostland/Settlements/Vault/Fixed/DA_Dilemma_Residence_Accessed_Final.DA_Dilemma_Residence_Accessed_Final")
    (`PXOutpostUtils.DestroyOutpost` _returnvalue)))