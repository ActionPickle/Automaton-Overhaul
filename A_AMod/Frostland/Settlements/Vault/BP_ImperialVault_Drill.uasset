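; Frostland logic for the Imperial Vault drill, turning completion of the final drilling stage into a dilemma.
; On start, it binds to the extraction subsystem's depletion update event.
; When the final vault drilling outpost is depleted, it spawns the vault-drilled dilemma at that outpost owner's transform, then destroys the outpost.
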(event `self.ReceiveStarted`
  (add `PXExtractionSubsystem.ExtractionDepletionUpdated` (subsystem `PXExtractionSubsystem`) (`|CreateDelegate` :!event `Door Drilled`)))

(event `Door Drilled`
  (params (extraction :type "PXExtractionComponent Object Reference"))
  (bind _returnvalue (`PXOutpostUtils.GetOutpostOfType` "/Game/Scenarios/Shared/Configs/A_AMod/Frostland/Settlements/Vault/Fixed/DA_Vault_Drilling_Final.DA_Vault_Drilling_Final"))
  (if (`PXOutpostUtils.IsOutpostDepleted` (`PXOutpostUtils.GetOutpostOfType` "/Game/Scenarios/Shared/Configs/A_AMod/Frostland/Settlements/Vault/Fixed/DA_Vault_Drilling_Final.DA_Vault_Drilling_Final"))
    (`PXDilemmaUtils.SpawnDilemma` (`Actor.GetTransform` (`ActorComponent.GetOwner` _returnvalue)) "/Game/Scenarios/Shared/Configs/A_AMod/Frostland/Settlements/Vault/Fixed/DA_Dilemma_Vault_Drilled.DA_Dilemma_Vault_Drilled")
    (`PXOutpostUtils.DestroyOutpost` _returnvalue)))